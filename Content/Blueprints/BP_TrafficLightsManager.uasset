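; Traffic light manager that cycles two groups of traffic lights through green, yellow and red, starting on BeginPlay.
; Each group tracks its own current color, advances every light in its array to the next one, then re-triggers itself after a Delay.
; Colors and per-color durations come from map lookups in ColorSettings and DelaySettings, applied through each light's ChangeColor.
; The two loops run independently, with no synchronization between groups.
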(event Custom|Recolor
  (Utilities|FlowControl|Sequence
    (:then_0
      (CallFunction|RecolorGroup1Event))
    (:then_1
      (CallFunction|RecolorGroup2Event))))

(event Custom|RecolorGroup2_Event
  (for _array_element (Variables|Group2|GetTrafficLightsGroup2)
    (switch Utilities|FlowControl|Switch|SwitchonE_LightColor (Variables|Group2|GetCurrentColorGroup2)
      (:NewEnumerator0
        (CallFunction|SetGreenColorEvent _array_element))
      (:NewEnumerator1
        (CallFunction|SetRedColorEvent _array_element))
      (:NewEnumerator2
        (CallFunction|SetYellowColorEvent _array_element))))
  (switch Utilities|FlowControl|Switch|SwitchonE_LightColor (Variables|Group2|GetCurrentColorGroup2)
    (:NewEnumerator0
      (Variables|Group2|SetCurrentColorGroup2 "NewEnumerator2"))
    (:NewEnumerator1
      (Variables|Group2|SetCurrentColorGroup2 "NewEnumerator0"))
    (:NewEnumerator2
      (Variables|Group2|SetCurrentColorGroup2 "NewEnumerator1")))
  (Utilities|FlowControl|Delay (.Value (Utilities|Map|Find (Utilities|Struct|BreakS_LIghtDelay (Variables|Settings|GetDelaySettings)) (Variables|Group2|GetCurrentColorGroup2))))
  (CallFunction|RecolorGroup2Event))

(event Custom|RecolorGroup1_Event
  (for _array_element (Variables|Group1|GetTrafficLightsGroup1)
    (switch Utilities|FlowControl|Switch|SwitchonE_LightColor (Variables|Group1|GetCurrentColorGroup1)
      (:NewEnumerator0
        (CallFunction|SetGreenColorEvent _array_element))
      (:NewEnumerator1
        (CallFunction|SetRedColorEvent _array_element))
      (:NewEnumerator2
        (CallFunction|SetYellowColorEvent _array_element))))
  (switch Utilities|FlowControl|Switch|SwitchonE_LightColor (Variables|Group1|GetCurrentColorGroup1)
    (:NewEnumerator0
      (Variables|Group1|SetCurrentColorGroup1 "NewEnumerator2"))
    (:NewEnumerator1
      (Variables|Group1|SetCurrentColorGroup1 "NewEnumerator0"))
    (:NewEnumerator2
      (Variables|Group1|SetCurrentColorGroup1 "NewEnumerator1")))
  (Utilities|FlowControl|Delay (.Value (Utilities|Map|Find (Utilities|Struct|BreakS_LIghtDelay (Variables|Settings|GetDelaySettings)) (Variables|Group1|GetCurrentColorGroup1))))
  (CallFunction|RecolorGroup1Event))

(event Custom|SetGreenColor_Event
  (params (TrafficLight :type BP%20Traffict%20Light%20Object%20Reference))
  (Default|ChangeColor TrafficLight (.Value (Utilities|Map|Find (Utilities|Struct|BreakS_LIghtColor (Variables|Settings|GetColorSettings)) "NewEnumerator2"))))

(event Custom|SetRedColor_Event
  (params (TrafficLight :type BP%20Traffict%20Light%20Object%20Reference))
  (Default|ChangeColor TrafficLight (.Value (Utilities|Map|Find (Utilities|Struct|BreakS_LIghtColor (Variables|Settings|GetColorSettings)) "NewEnumerator0"))))

(event Custom|SetYellowColor_Event
  (params (TrafficLight :type BP%20Traffict%20Light%20Object%20Reference))
  (Default|ChangeColor TrafficLight (.Value (Utilities|Map|Find (Utilities|Struct|BreakS_LIghtColor (Variables|Settings|GetColorSettings)) "NewEnumerator1"))))

(event EventBeginPlay
  (CallFunction|Recolor))

(fn ConstructionScript)